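; Item Blueprint that shows an interaction prompt while a MissPBCharacter stands inside its Box trigger.
; Begin overlap sets the character's IsOverlappingItem flag, creates an Interact widget, passes it to SetItemName and adds it to the viewport.
; End overlap clears the flag and removes every top-level Interact widget, including any created by other items.
; SetItemName is an empty function here, so the widget receives no name from this Blueprint.
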(event `self.Box.OnComponentBeginOverlap`
  (params (OverlappedComponent :type "PrimitiveComponent Object Reference") (OtherActor :type "Actor Object Reference") (OtherComp :type "PrimitiveComponent Object Reference") (OtherBodyIndex :type Integer) (bFromSweep :type Boolean) (SweepResult :type "HitResult Structure (by ref)"))
  (bind _asmiss_pbcharacter (cast `MissPBCharacter` OtherActor))
  (set `MissPBCharacter.isOverlappingItem` true _asmiss_pbcharacter)
  (bind _returnvalue (`|CreateWidget` "/Game/Items/Widgets/Interact.Interact_C"))
  (`self.SetItemName` _returnvalue)
  (`UserWidget.AddToViewport` _returnvalue 0))

(event `self.Box.OnComponentEndOverlap`
  (params (OverlappedComponent :type "PrimitiveComponent Object Reference") (OtherActor :type "Actor Object Reference") (OtherComp :type "PrimitiveComponent Object Reference") (OtherBodyIndex :type Integer))
  (bind _asmiss_pbcharacter (cast `MissPBCharacter` OtherActor))
  (set `MissPBCharacter.isOverlappingItem` false _asmiss_pbcharacter)
  (bind _foundwidgets (`WidgetBlueprintLibrary.GetAllWidgetsOfClass` "/Game/Items/Widgets/Interact.Interact_C"))
  (for _array_element _foundwidgets
    (`Widget.RemoveFromParent` _array_element)))

(fn `SetItemName`
  (params (WidgetRef :type "/Game/Items/Widgets/Interact Object Reference")))

(fn `UserConstructionScript`)